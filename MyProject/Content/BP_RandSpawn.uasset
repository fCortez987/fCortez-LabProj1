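; BP_RandSpawn is a spawner that periodically drops random items at target points in the level.
; BeginPlay caches all TargetPoint actors and starts a looping timer with a random interval chosen once.
; Each tick of that timer has roughly even odds of spawning a random Drops class at a random point or printing a miss message.
; The re-rolled RandTime never updates the timer, and an all-points spawn loop is left unconnected.
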(event Custom|Spawn%20Things
  (bind _spawnposition (Variables|Default|GetSpawnPosition))
  (bind _output_get (Variables|Default|SetrandTime (Math|Random|RandomFloatinRange 0.01 4e+02)))
  (if (> (Math|Random|RandomIntegerinRange 0 100) 50)
    (Game|SpawnActorfromClass (.OutItem (Utilities|Array|Random (Variables|Default|Getdrops))) (Transformation|GetActorTransform (Utilities|Array|Get(acopy) _spawnposition (Math|Random|RandomIntegerinRange 0 (- (Utilities|Array|Length _spawnposition) 1)))) "Undefined" "MultiplyWithRoot" 0 0)
    (else
      (Development|PrintString "YOU GET NOTHING"))))

(event EventBeginPlay
  (bind _outactors (Actor|GetAllActorsOfClass "/Script/Engine.TargetPoint"))
  (Variables|Default|SetSpawnPosition _outactors)
  (Variables|Default|SetrandTime (Math|Random|RandomFloatinRange 1.0 3.0))
  (Utilities|Time|SetTimerbyFunctionName 0 "Spawn Things" (stale Custom|Spawn%20Things _output_get) true true))

(fn ConstructionScript
  (|CallParentFunction))